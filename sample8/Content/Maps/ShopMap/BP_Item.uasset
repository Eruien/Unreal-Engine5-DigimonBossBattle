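; BP_Item is an item actor in the shop map that takes its skeletal mesh from the ItemList data table.
; On BeginPlay it loops over three index-named rows, storing each found row in ItemInfo and requesting an async load of its mesh.
; A completed load increments ItemID and applies the mesh to the single SkeletalMesh component.
; Overlap, Tick and the construction script are empty.
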(event EventBeginPlay
  (for _index (range 0 2)
    (bind _returnvalue (Utilities|GetDataTableRow "/Game/Maps/ShopMap/ItemList.ItemList" (Utilities|String|StringToName (Utilities|String|ToString(Integer) _index)))
      (:then
        (bind _output_get (Variables|Default|SetItemInfo _returnvalue))
        (bind _object (Utilities|AsyncLoadAsset (.Mesh (Utilities|Struct|BreakItem _output_get)))
          (:Completed
            (Variables|Default|SetItemID (+ (Variables|Default|GetItemID) 1))
            (bind _as스켈레탈_메시 (Utilities|Casting|CastToSkeletalMesh _object))
            (Components|SkinnedMesh|SetSkinnedAssetandUpdate (Variables|Default|GetSkeletalMesh) _as스켈레탈_메시 true)))))))

(event Collision|EventActorBeginOverlap
  (params (OtherActor :type Actor%20Object%20Reference)))

(event EventTick
  (params (DeltaSeconds :type Float%20%28single-precision%29)))

(fn ConstructionScript)