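; BP_Test is a test actor that acts like an item pickup, reacting to overlaps on its static mesh.
; Each overlap begin toggles the actor's hidden-in-game state, then calls ItemGain.
; ItemGain decrements ItemCount on BP_IngameGamemode and prints a debug string.
; The actor is never destroyed and overlaps are not filtered, so repeat overlaps flip visibility and decrement again.
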(event OnComponentBeginOverlap(StaticMesh)
  (params (OverlappedComponent :type Primitive%20Component%20Object%20Reference) (OtherActor :type Actor%20Object%20Reference) (OtherComp :type Primitive%20Component%20Object%20Reference) (OtherBodyIndex :type Integer) (bFromSweep :type Boolean) (SweepResult :type Hit%20Result%20Structure%20%28by%20ref%29))
  (bind _output_get (Variables|Default|SetHiddenMode (not (Variables|Default|GetHiddenMode))))
  (Rendering|SetActorHiddenInGame _output_get)
  (CallFunction|ItemGain))

(event EventBeginPlay)

(event Collision|EventActorBeginOverlap
  (params (OtherActor :type Actor%20Object%20Reference)))

(event EventTick
  (params (DeltaSeconds :type Float%20%28single-precision%29)))

(fn ConstructionScript)

(fn ItemGain
  (bind _asbp_ingame_gamemode (Utilities|Casting|CastToBP_IngameGamemode (Game|GetGameMode)))
  (bind _result (Math|Integer|DecrementInt (Variables|/Game/Map/BP_IngameGamemode.BP_IngameGamemode_C|GetitemCount _asbp_ingame_gamemode))
    (:%20%20
      (Variables|/Game/Map/BP_IngameGamemode.BP_IngameGamemode_C|SetitemCount _asbp_ingame_gamemode _result)
      (Development|PrintString "fucn"))))