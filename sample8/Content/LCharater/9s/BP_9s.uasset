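; BP_9s is the player character 9s, with montage-driven combo slash, dash and roll, and it shows the main UI widget on BeginPlay.
; Left click starts the combo unless already playing, while right click and Left Shift play dash and roll.
; Tick snaps actor yaw to control rotation during the combo.
; 9sSlashRay box-traces between two sword sockets, returning hit result and actor, with debug drawing.
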(event EventBeginPlay
  (bind _asui_instance (Utilities|Casting|CastToUI_Instance (Game|GetGameInstance)))
  (Default|ShowMainWidget _asui_instance true))

(event Collision|EventActorBeginOverlap
  (params (OtherActor :type Actor%20Object%20Reference)))

(event EventTick
  (params (DeltaSeconds :type Float%20%28single-precision%29))
  (bind _mesh (Variables|Character|GetMesh))
  (bind _returnvalue (Components|SkeletalMesh|GetAnimInstance _mesh))
  (Variables|Default|SetAttackRotation (Class|AnimInstance|MontageGetIsStopped _returnvalue "/Game/LCharater/9s/Montage/MT_ComboSlash.MT_ComboSlash"))
  (if (Animation|Montage|MontageIsPlaying _returnvalue "/Game/LCharater/9s/Montage/MT_ComboSlash.MT_ComboSlash")
    (Transformation|SetActorRotation (Math|Rotator|MakeRotator 0.0 0.0 (.yaw (Pawn|GetControlRotation :!class /Script/Engine.Pawn))))))

(event Input|MouseEvents|RightMouseButton
  (params (Key :type Key%20Structure :default "None"))
  (:Pressed
    (Animation|Montage|PlayMontage (Variables|Character|GetMesh) "/Game/LCharater/9s/Montage/MT_Dash.MT_Dash")))

(event Input|MouseEvents|LeftMouseButton
  (params (Key :type Key%20Structure :default "None"))
  (:Pressed
    (Variables|Default|SetLeftMouseClick true)
    (if (not (Animation|Montage|MontageIsPlaying (Components|SkeletalMesh|GetAnimInstance (Variables|Character|GetMesh)) "/Game/LCharater/9s/Montage/MT_ComboSlash.MT_ComboSlash"))
      (Animation|Montage|PlayMontage (Variables|Character|GetMesh) "/Game/LCharater/9s/Montage/MT_ComboSlash.MT_ComboSlash" 1.0 0.0 ""
        (:then
          (Variables|Default|SetLeftMouseClick false))))))

(event Input|KeyboardEvents|LeftShift
  (params (Key :type Key%20Structure :default "None"))
  (:Pressed
    (Animation|Montage|PlayMontage (Variables|Character|GetMesh) "/Game/LCharater/9s/Montage/MT_Roll.MT_Roll")))

(fn ConstructionScript)

(fn 9sSlashRay
  (bind _mesh (Variables|Character|GetMesh))
  (bind (_outhit _returnvalue) (Collision|BoxTraceByChannel (Transformation|GetSocketLocation _mesh "SwordRay0") (Transformation|GetSocketLocation _mesh "SwordRay1") "10.000000,10.000000,0.000000" "0, 0, 0" "TraceTypeQuery1" false 0 "ForDuration"))
  (return _returnvalue (.HitActor (Collision|BreakHitResult _outhit))))